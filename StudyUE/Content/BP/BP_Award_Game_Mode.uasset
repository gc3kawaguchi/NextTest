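; Game mode for the Award game that handles player respawn, stage streaming and the play UI.
; On BeginPlay it binds pawn respawn, loads the current stage, adds the W_Play widget and resets life, item and clear state in the game instance.
; A destroyed pawn is replaced by a possessed BP_Award at the player start, rebinding the handler.
; Stage advance increments the level name's numeric suffix, swaps streamed levels and repositions the pawn.
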(event Custom|RespawnIvent
  (bind _returnvalue (Game|Player|GetPlayerPawn 0))
  (Utilities|IsValid _returnvalue
    (:Is%20Valid
      (Game|AssignOnDestroyed _returnvalue (delegate Custom|RespawnAward)))))

(event Custom|RespawnAward
  (params (DestroyedActor :type Actor%20Object%20Reference))
  (bind _returnvalue (Game|SpawnActorfromClass "/Game/BP/BP_Award.BP_Award_C" (Transformation|GetActorTransform (Class|GameModeBase|FindPlayerStart)) "Undefined" 0 0))
  (Pawn|Possess (Game|GetPlayerController 0) _returnvalue)
  (CallFunction|RespawnIvent))

(event Custom|CreateUI
  (bind _returnvalue (UserInterface|CreateWidget "/Game/UI/W_Play.W_Play_C"))
  (UserInterface|Viewport|AddtoViewport _returnvalue 0))

(event Custom|LoadStage
  (Game|LoadStreamLevel(byName) (Variables|Default|GetStage_name) true true)
  (CallFunction|SetAwardTransform))

(event Custom|inityal_game_instance
  (bind _returnvalue (Game|GetGameInstance))
  (bind _asaward_game_instance (Utilities|Casting|CastToAward_Game_instance _returnvalue))
  (Variables|/Game/BP/Award_Game_instance.Award_Game_instance_C|Setlife _asaward_game_instance 2)
  (Variables|/Game/BP/Award_Game_instance.Award_Game_instance_C|Setis_clere _asaward_game_instance false)
  (Variables|/Game/BP/Award_Game_instance.Award_Game_instance_C|Setitem _asaward_game_instance 0))

(event Custom|next_stage
  (Game|UnloadStreamLevel(byName) (Variables|Default|GetStage_name) false)
  (bind _output_get (Variables|Default|SetStage_name (Utilities|String|StringToName (Utilities|String|Append (Utilities|String|Left (Utilities|String|ToString(Name) (Variables|Default|GetStage_name)) 6) (Utilities|String|ToString(Integer) (+ (Math|Conversions|ToInteger(Byte) (Utilities|String|RightChop (Utilities|String|ToString(Name) (Variables|Default|GetStage_name)) 6)) 1))))))
  (Game|LoadStreamLevel(byName) _output_get true true)
  (CallFunction|SetAwardTransform))

(event EventBeginPlay
  (CallFunction|RespawnIvent)
  (CallFunction|LoadStage)
  (CallFunction|CreateUI)
  (CallFunction|InityalGameInstance)
  (Development|PrintString "Hello"))

(event EventTick
  (params (DeltaSeconds :type Float%20%28single-precision%29)))

(fn ConstructionScript)

(fn SetAwardTransform
  (Transformation|SetActorTransform (Game|Player|GetPlayerPawn 0) (Transformation|GetActorTransform (Class|GameModeBase|FindPlayerStart))))