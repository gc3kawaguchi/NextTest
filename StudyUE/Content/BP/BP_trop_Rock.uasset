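; Rock spawner that periodically launches BP_Rock actors from a hole wall, likely as a level hazard.
; A looping timer spawns each rock at an offset from the Arrow, enables physics and applies a velocity-change impulse along the Arrow's forward axis.
; The construction script adds an end wall mesh at HoleWallEndLocation, rotating both walls to face each other.
; Rocks ending overlap with Foll_wall_end get a short lifespan.
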(event OnComponentEndOverlap(foll_wall_end)
  (params (OverlappedComponent :type Primitive%20Component%20Object%20Reference) (OtherActor :type Actor%20Object%20Reference) (OtherComp :type Primitive%20Component%20Object%20Reference) (OtherBodyIndex :type Integer))
  (bind _asbp_rock (Utilities|Casting|CastToBP_Rock OtherActor))
  (Actor|SetLifeSpan _asbp_rock 1.0))

(event Custom|SpawnRock
  (bind _arrow (Variables|Default|GetArrow))
  (bind _returnvalue (Transformation|GetWorldTransform _arrow))
  (bind (_location _rotation _scale) (Math|Transform|BreakTransform _returnvalue))
  (bind _returnvalue_2 (Game|SpawnActorfromClass "/Game/BP/BP_Rock.BP_Rock_C" (Math|Transform|MakeTransform (Math|Transform|TransformLocation _returnvalue "100.000000, 0,-100.000000") _rotation _scale) "Undefined" 0 0))
  (Physics|SetSimulatePhysics (Variables|/Game/BP/BP_Rock.BP_Rock_C|Getrock_mesh _returnvalue_2) true)
  (Physics|AddImpulse (Variables|/Game/BP/BP_Rock.BP_Rock_C|Getrock_mesh _returnvalue_2) (Math|Transform|TransformDirection _returnvalue "1000.000000, 0, 0") "None" true))

(event EventBeginPlay
  (Utilities|Time|SetTimerbyEvent (delegate Custom|SpawnRock) 3.0 true))

(event Collision|EventActorBeginOverlap
  (params (OtherActor :type Actor%20Object%20Reference)))

(event EventTick
  (params (DeltaSeconds :type Float%20%28single-precision%29)))

(fn ConstructionScript
  (bind _hole_wall_end_location (Variables|Default|Gethole_wall_end_location))
  (bind _holewallstert (Variables|Default|GetHoleWallStert))
  (bind _relativelocation (Variables|/Script/Engine.SceneComponent|GetRelativeLocation _holewallstert))
  (Transformation|SetRelativeRotation _holewallstert (Math|Rotator|FindLookatRotation _relativelocation _hole_wall_end_location) false false)
  (bind _returnvalue (AddComponent|AddStaticMeshComponent false (Math|Transform|MakeTransform _hole_wall_end_location (Math|Rotator|FindLookatRotation _hole_wall_end_location _relativelocation))))
  (Variables|Default|Setfoll_wall_end _returnvalue))